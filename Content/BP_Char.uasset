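; BP_Char is the player character with movement, look, interaction and a time-reverse ability.
; Axis inputs drive forward and strafe movement along the actor's vectors, plus controller yaw and pitch.
; Holding the reverse action begins time reversal through the TimeManager of ReverseTime, and releasing it ends it.
; The Interact press forwards to CallAction on PressableSource.
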(event Collision|EventActorBeginOverlap
  (params (OtherActor :type Actor%20Object%20Reference)))

(event EventTick
  (params (DeltaSeconds :type Float%20%28single-precision%29)))

(event Input|ActionEvents|InputActionreverse
  (params (Key :type Key%20Structure :default "None"))
  (bind _reversetime (Variables|Default|GetReverseTime))
  (bind _timemanager (Variables|/Script/TimePower1.ReverseTimeComponent|GetTimeManager _reversetime))
  ;[1 1 1] 2
  (:Pressed
    (Class|TimeManager|BeginTimeReverse _timemanager))
  (:Released
    (Class|TimeManager|EndTimeReverse _timemanager)))

(event Input|ActionEvents|InputActionInteract
  (params (Key :type Key%20Structure :default "None"))
  (:Pressed
    (Default|CallAction (Variables|Default|GetPressableSource))))

(event Input|AxisEvents|InputAxisMFWD
  (params (AxisValue :type Float%20%28single-precision%29))
  ;[1 1 1] 1
  (Pawn|Input|AddMovementInput (Transformation|GetActorForwardVector) AxisValue false))

(event Input|AxisEvents|InputAxisMRIGHT
  (params (AxisValue :type Float%20%28single-precision%29))
  ;[1 1 1] 1
  (Pawn|Input|AddMovementInput (Transformation|GetActorRightVector) AxisValue false))

(event Input|AxisEvents|InputAxisLOOkUP
  (params (AxisValue :type Float%20%28single-precision%29))
  ;[1 1 1] 1
  (Pawn|Input|AddControllerPitchInput AxisValue))

(event Input|AxisEvents|InputAxisLOOKROUND
  (params (AxisValue :type Float%20%28single-precision%29))
  ;[1 1 1] 1
  (Pawn|Input|AddControllerYawInput AxisValue))

(fn ConstructionScript)
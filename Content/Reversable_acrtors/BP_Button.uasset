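; BP_Button is a button actor that visibly sinks when its pressable action fires.
; Box overlap events register and unregister pawns with the PressableAction component.
; That component's Action event offsets the Button component downward without sweeping and sets an ISPressed flag so it moves only once.
; The graph contains no logic to raise the button or clear the flag.
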(event OnComponentBeginOverlap(Box)
  (params (OverlappedComponent :type Primitive%20Component%20Object%20Reference) (OtherActor :type Actor%20Object%20Reference) (OtherComp :type Primitive%20Component%20Object%20Reference) (OtherBodyIndex :type Integer) (bFromSweep :type Boolean) (SweepResult :type Hit%20Result%20Structure%20%28by%20ref%29))
  (bind _aspawn (Utilities|Casting|CastToPawn OtherActor))
  (Default|RegisterCharacter (Variables|Default|GetPressableAction) _aspawn))

(event OnComponentEndOverlap(Box)
  (params (OverlappedComponent :type Primitive%20Component%20Object%20Reference) (OtherActor :type Actor%20Object%20Reference) (OtherComp :type Primitive%20Component%20Object%20Reference) (OtherBodyIndex :type Integer))
  (bind _aspawn (Utilities|Casting|CastToPawn OtherActor))
  (Default|UnregisterCharacter (Variables|Default|GetPressableAction) _aspawn))

(event Action(PressableAction)
  (if (== (Variables|Default|GetISPressed) false)
    (Transformation|AddLocalOffset (Variables|Default|GetButton) "0.000000,0.000000,-20.000000" false false)
    (Variables|Default|SetISPressed true)))

(event EventBeginPlay)

(event Collision|EventActorBeginOverlap
  (params (OtherActor :type Actor%20Object%20Reference)))

(event EventTick
  (params (DeltaSeconds :type Float%20%28single-precision%29)))

(fn ConstructionScript)